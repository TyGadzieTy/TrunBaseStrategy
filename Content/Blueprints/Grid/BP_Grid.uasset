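; BP_Grid is a grid actor that builds a field of flat square tiles from a position, tile size and grid size.
; The construction script calls SpawnGrid, which sets the square mesh and border material on the instanced GridMesh.
; A nested X/Y loop adds one scaled instance per cell, offset from a corner computed to center the grid on the position.
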(fn `SpawnGrid`
  (params (Position :type "Vector Structure") (TileSize :type "Vector Structure") (`Grid Size` :type "Vector2D Structure"))
  (locals (XIndex :type Integer) (YIndex :type Integer) (`Tile Transform Position` :type "Transform Structure"))
  (bind _grid_mesh (`self.Grid Mesh`))
  (bind (_grid_size_x _grid_size_y) (`KismetMathLibrary.BreakVector2D` (`self.Grid Size`)))
  (bind _grid_size_x_2 (`KismetMathLibrary.BreakVector2D` (`self.Grid Size`)))
  (set `self.Position` Position)
  (set `self.Tile Size` TileSize)
  (set `self.Grid Size` `Grid Size`)
  (`StaticMeshComponent.SetStaticMesh` _grid_mesh "/Game/Assets/Meshes/Grid/SM_Grid_SquareFlat.SM_Grid_SquareFlat")
  (`PrimitiveComponent.SetMaterial` _grid_mesh 0 "/Game/Assets/Materials/Grid/MI_GridBorder.MI_GridBorder")
  (set `self.GridLeftCornerLocation` (- (`self.Position`) (`KismetMathLibrary.Conv_Vector2DToVector` (* (/ (`self.Grid Size`) 2.0) (`KismetMathLibrary.Conv_VectorToVector2D` (`self.Tile Size`))))))
  (for _index (range (`KismetMathLibrary.Round` _grid_size_x_2))
    (set `local.XIndex` _index)
    (for _index_2 (range (`KismetMathLibrary.Round` _grid_size_y))
      (set `local.YIndex` _index_2)
      (set `local.Tile Transform Position` (`KismetMathLibrary.MakeTransform` (+ (`self.GridLeftCornerLocation`) (* (`self.Tile Size`) (`KismetMathLibrary.MakeVector` (`KismetMathLibrary.Conv_IntToDouble` (`local.XIndex`)) (`KismetMathLibrary.Conv_IntToDouble` (`local.YIndex`))))) (struct) (/ (`self.Tile Size`) (100.0 100.0 1.0))))
      (`InstancedStaticMeshComponent.AddInstance` (`self.Grid Mesh`) (`local.Tile Transform Position`)))))

(fn `UserConstructionScript`
  (`self.SpawnGrid` (`self.Position`) (`self.Tile Size`) (`self.Grid Size`)))
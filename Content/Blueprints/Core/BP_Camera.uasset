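; BP_Camera is a camera Blueprint that rotates in yaw steps on player input.
; The RotateCameraLeft and RotateCameraRight press events add or subtract CameraRotationValue from the scene root's current world yaw.
; Each press sets the new rotation immediately, with no interpolation, and the construction script is empty.
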(event `InputAction|RotateCameraLeft`
  (params (Key :type "Key Structure"))
  (bind _defaultsceneroot (`self.DefaultSceneRoot`))
  (bind (_returnvalue_roll _returnvalue_pitch _returnvalue_yaw) (`KismetMathLibrary.BreakRotator` (`SceneComponent.K2_GetComponentRotation` _defaultsceneroot)))
  ;[1 1 1] Camera Rotation
  (:`Pressed`
    (`SceneComponent.K2_SetWorldRotation` _defaultsceneroot (`KismetMathLibrary.MakeRotator` 0.0 0.0 (+ _returnvalue_yaw (`self.Camera Rotation Value`))) false false)))

(event `InputAction|RotateCameraRight`
  (params (Key :type "Key Structure"))
  (bind _defaultsceneroot (`self.DefaultSceneRoot`))
  (bind (_returnvalue_roll _returnvalue_pitch _returnvalue_yaw) (`KismetMathLibrary.BreakRotator` (`SceneComponent.K2_GetComponentRotation` _defaultsceneroot)))
  ;[1 1 1] Camera Rotation
  (:`Pressed`
    (`SceneComponent.K2_SetWorldRotation` _defaultsceneroot (`KismetMathLibrary.MakeRotator` 0.0 0.0 (- _returnvalue_yaw (`self.Camera Rotation Value`))) false false)))

(fn `UserConstructionScript`)